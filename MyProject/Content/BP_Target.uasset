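; BP_Target is an interactable trigger that lets the first-person player raise and lower a box once their Count reaches three.
; Overlap shows Lightbulb1 and enables input; leaving hides it and disables input.
; Pressing F below that count prints a warning; otherwise a FlipFlop alternates two timelines lerping Box between hardcoded world positions.
; Input is disabled during each move and re-enabled on finish.
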(event EventBeginPlay
  (Rendering|SetActorHiddenInGame (Variables|Components|GetLightbulb1) true)
  (bind _asbp_first_person_character (Utilities|Casting|CastToBP_FirstPersonCharacter (Game|Player|GetPlayerPawn 0)))
  (Variables|Default|SetPlayer1 _asbp_first_person_character))

(event Collision|EventActorEndOverlap
  (params (OtherActor :type Actor%20Object%20Reference))
  (Utilities|Casting|CastToBP_FirstPersonCharacter OtherActor)
  (Input|DisableInput (Game|GetPlayerController 0))
  (Rendering|SetActorHiddenInGame (Variables|Components|GetLightbulb1) true))

(event Collision|EventActorBeginOverlap
  (params (OtherActor :type Actor%20Object%20Reference))
  (Utilities|Casting|CastToBP_FirstPersonCharacter OtherActor)
  (Rendering|SetActorHiddenInGame (Variables|Components|GetLightbulb1) false)
  (Input|EnableInput (Game|GetPlayerController 0)))

(event Input|KeyboardEvents|F
  (params (Key :type Key%20Structure :default "None"))
  (bind _returnvalue (Game|GetPlayerController 0))
  (bind _returnvalue_2 (Game|GetPlayerController 0))
  (bind _box (Variables|Default|GetBox))
  (:Pressed
    (if (> (Variables|/Game/FirstPerson/Blueprints/BP_FirstPersonCharacter.BP_FirstPersonCharacter_C|GetCount (Variables|Default|GetPlayer1)) 2)
      (Utilities|FlowControl|FlipFlop
        (:A
          (Development|PrintString "Up!")
          (Input|DisableInput _returnvalue)
          (bind _movement_delta (Timeline|Timeline Play)
            (:Update
              (Transformation|SetWorldLocation _box (Math|Vector|Lerp(Vector) "1680.000000,2340.000000,30.000000" "1680.000000,2340.000000,300.000000" _movement_delta) false false))
            (:Finished
              (Input|EnableInput _returnvalue_2))))
        (:B
          (Development|PrintString "Down!")
          (Input|DisableInput _returnvalue)
          (bind _movement_delta_2 (Timeline|Timeline_0 Play)
            (:Update
              (Transformation|SetWorldLocation _box (Math|Vector|Lerp(Vector) "1680.000000,2340.000000,300.000000" "1680.000000,2340.000000,30.000000" _movement_delta_2) false false))
            (:Finished
              (Input|EnableInput _returnvalue_2)))))
      (else
        (Development|PrintString "You need at least Three points!")))))

(fn ConstructionScript)