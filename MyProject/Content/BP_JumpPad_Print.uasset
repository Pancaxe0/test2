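; Jump pad variant that spawns a BP_Cube at its Pad component's location when an actor overlaps it.
; The overlap event runs the parent's handler first, then checks the Closed flag.
; A DoOnce clears Closed on the first overlap that finds it set, followed by a short delay.
; The construction script only calls the parent's.
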(event Collision|EventActorBeginOverlap
  (params (OtherActor :type Actor%20Object%20Reference))
  (|CallParentFunction OtherActor)
  (if (Variables|Default|GetClosed)
    (Utilities|FlowControl|DoOnce false
      (:Completed
        (Variables|Default|SetClosed false)
        (Utilities|FlowControl|Delay 3.0))))
  (Game|SpawnActorfromClass "/Game/BP_Cube.BP_Cube_C" (Math|Conversions|ToTransform(Vector) (Transformation|GetWorldLocation (Variables|Default|GetPad))) "Undefined" "MultiplyWithRoot" 0 0))

(fn ConstructionScript
  (|CallParentFunction))