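; Pickup actor that adds one to the first-person player character's Count when hit, then destroys itself.
; BeginPlay casts the first player pawn to BP_FirstPersonCharacter and caches it as Player.
; The Hit event increments Count on that cached reference without checking what hit it, and prints debug text with the count before destruction.
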(event EventBeginPlay
  (bind _asbp_first_person_character (Utilities|Casting|CastToBP_FirstPersonCharacter (Game|Player|GetPlayerPawn 0)))
  (Variables|Default|SetPlayer _asbp_first_person_character))

(event Collision|EventHit
  (params (MyComp :type Primitive%20Component%20Object%20Reference) (Other :type Actor%20Object%20Reference) (OtherComp :type Primitive%20Component%20Object%20Reference) (bSelfMoved :type Boolean) (HitLocation :type Vector :default "0, 0, 0") (HitNormal :type Vector :default "0, 0, 0") (NormalImpulse :type Vector :default "0, 0, 0") (Hit :type Hit%20Result%20Structure%20%28by%20ref%29))
  (bind _result (Math|Integer|IncrementInt (Variables|/Game/FirstPerson/Blueprints/BP_FirstPersonCharacter.BP_FirstPersonCharacter_C|GetCount (Variables|Default|GetPlayer)))
    (:%20%20
      (Development|PrintString "Hit!")
      (Development|PrintString (Utilities|String|ToString(Integer) _result))
      (Actor|DestroyActor))))

(fn ConstructionScript)